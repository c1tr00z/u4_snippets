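; Base character Blueprint with two movement helpers: a rotate-to-angle event and a movement input check.
; E_RotateToAngle makes one RInterpTo step of the controller's rotation toward a target yaw, with zero pitch and roll and a fixed delta time.
; CanMove tests the two-axis input's magnitude against a dead zone, returning that magnitude as speed scale and the actor's flattened, normalized forward vector as direction.
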(event Custom|E_RotateToAngle
  (params (TargetAngle :type Float%20%28single-precision%29))
  (bind _returnvalue (Pawn|GetController))
  (Pawn|SetControlRotation _returnvalue (Math|Interpolation|RInterpTo (Pawn|GetControlRotation _returnvalue :!class /Script/Engine.Controller) (Math|Rotator|MakeRotator 0.0 0.0 TargetAngle) 0.5 0.15)))

(event EventBeginPlay)

(event Collision|EventActorBeginOverlap
  (params (OtherActor :type Actor%20Object%20Reference)))

(event EventTick
  (params (DeltaSeconds :type Float%20%28single-precision%29)))

(fn ConstructionScript)

(fn CanMove
  (params (XValue :type Float%20%28single-precision%29) (YValue :type Float%20%28single-precision%29))
  (bind _returnvalue (Math|Vector2D|MakeVector2D XValue YValue))
  (bind _returnvalue_2 (Math|Vector2D|Vector2DLength _returnvalue))
  (return (> _returnvalue_2 0.25) (Math|Conversions|ToVector(Vector2D) (Math|Vector2D|Normalize2D (Math|Conversions|ToVector2D(Vector) (Transformation|GetActorForwardVector)))) _returnvalue_2))